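; NPC_AI_BP is an NPC AI controller that runs guard behavior and picks enemies through AI perception.
; On BeginPlay it sets up Patrol_Blackboard and runs the GuardBehaviour_BT behavior tree.
; Perception updates write sensed actors lacking the AntiPlayerEnemyFaction tag into the blackboard's EnemyKey.
; A failed sense of any such actor clears that key, whether or not it is the stored enemy.
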(event `self.ReceiveBeginPlay`
  (`self.UseBlackboard` "/Game/Dynamic/NPC/AI/Patrol_Blackboard.Patrol_Blackboard")
  (`self.RunBehaviorTree` "/Game/Dynamic/NPC/AI/GuardBehaviour_BT.GuardBehaviour_BT"))

(event `self.AIPerception.OnTargetPerceptionUpdated`
  (params (Actor :type "Actor Object Reference") (Stimulus :type "AIStimulus Structure"))
  (bind _returnvalue (`AIBlueprintHelperLibrary.GetBlackboard` null))
  (bind _enemykey (`self.EnemyKey`))
  (if (`self.ActorHasTag` Actor "AntiPlayerEnemyFaction")
    _
    (elif (`.bSuccessfullySensed` (break `AIStimulus` Stimulus))
      (`BlackboardComponent.SetValueAsObject` _returnvalue _enemykey Actor)
      (else
        (`BlackboardComponent.ClearValue` _returnvalue _enemykey)))))

(fn `UserConstructionScript`)